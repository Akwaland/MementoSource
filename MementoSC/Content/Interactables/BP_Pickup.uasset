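; BP_Pickup is a world item pickup that the player can add to their inventory.
; The construction script loads its item row from a data table and sets the mesh, and BeginPlay labels the name plate.
; Overlap with BP_VictorianCharacter shows or hides the plate and switches input.
; E adds the item and destroys the pickup on success, while R removes that item and quantity.
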(event `self.ReceiveBeginPlay`
  ;[1 1 1] Update the name plate (Can't be done in construction script due to 'Get User Widget Object' node.
  (bind _aswg_pickup_name_plate (cast `/Game/Interactables/WG_PickupNamePlate` (`WidgetComponent.GetUserWidgetObject` (`self.NamePlate`))))
  (`TextBlock.SetText` (`/Game/Interactables/WG_PickupNamePlate.NameText` _aswg_pickup_name_plate) (`KismetTextLibrary.Conv_StringToText` (`KismetStringLibrary.Concat_StrStr` "[E]" (`KismetStringLibrary.Conv_NameToString` (`.Names_9_B48A52A94455017AEC171590E0AFA9BE` (break `/Game/Structures/ST_items` (`self.information`))))))))

(event `self.InteractionCollider.OnComponentBeginOverlap`
  (params (OverlappedComponent :type "PrimitiveComponent Object Reference") (OtherActor :type "Actor Object Reference") (OtherComp :type "PrimitiveComponent Object Reference") (OtherBodyIndex :type Integer) (bFromSweep :type Boolean) (SweepResult :type "HitResult Structure (by ref)"))
  ;[1 1 1] Show nameplate and enable input events when the player is inside/ touching the interactionCollider
  (if (`KismetMathLibrary.ClassIsChildOf` (`GameplayStatics.GetObjectClass` OtherActor) "/Game/VHExterior/Blueprints/BP_VictorianCharacter.BP_VictorianCharacter_C")
    (`SceneComponent.SetVisibility` (`self.NamePlate`) true false)
    (`self.EnableInput` (`GameplayStatics.GetPlayerController` 0))))

(event `self.InteractionCollider.OnComponentEndOverlap`
  (params (OverlappedComponent :type "PrimitiveComponent Object Reference") (OtherActor :type "Actor Object Reference") (OtherComp :type "PrimitiveComponent Object Reference") (OtherBodyIndex :type Integer))
  ;[1 1 1] Hide nameplate and enable input events when the player is inside/ touching the interactionCollider
  (if (`KismetMathLibrary.ClassIsChildOf` (`GameplayStatics.GetObjectClass` OtherActor) "/Game/VHExterior/Blueprints/BP_VictorianCharacter.BP_VictorianCharacter_C")
    (`SceneComponent.SetVisibility` (`self.NamePlate`) false false)
    (`self.DisableInput` (`GameplayStatics.GetPlayerController` 0) null)))

(event `Key|E`
  (params (Key :type "Key Structure"))
  ;[1 1 1] Add the item pulled from our database
  (:`Pressed`
    (bind _successfullyadded (`/Game/libraries/BPL_InventoryLibrary.AddItem` (`self.information`) (`.Quantity_24_EC06EEC741506C802F667E871BDA30A0` (break `/Game/Structures/ST_items` (`self.information`)))))
    ;[1 1 1] if the add was successful, destroy this pickup
    (if _successfullyadded
      (`self.K2_DestroyActor`))))

(event `Key|R`
  (params (Key :type "Key Structure"))
  ;[1 1 1] rEMOVE the item pulled from our database
  (:`Pressed`
    (`/Game/libraries/BPL_InventoryLibrary.RemoveItem` (`self.information`) (`.Quantity_24_EC06EEC741506C802F667E871BDA30A0` (break `/Game/Structures/ST_items` (`self.information`))))))

(fn `UserConstructionScript`
  (bind (_datatable _rowname) (break `DataTableRowHandle` (`self.item`)))
  ;[1 1 1] Get the ST_Item structure that corresponds with the row-specified in the 'item' variable, and assign it to our 'information' variable
  (bind _returnvalue (`|GetDataTableRow` _datatable _rowname)
    (:`then`
      (set `self.information` _returnvalue)
      ;[1 1 1] Update the mesh to whatever is defined in our 'information variable
      (`StaticMeshComponent.SetStaticMesh` (`self.Model`) (`.Model_26_C5643C8D4B3DAA46CF898EAD8E464FA5` (break `/Game/Structures/ST_items` (`self.information`)))))))